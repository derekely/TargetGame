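; Game mode for a timed target game, where the player wins by reaching a score equal to the number of targets before time runs out.
; BeginPlay counts BP_Target actors as the max score, creates the HUD widget and starts a fast looping countdown timer.
; AddScore and the countdown update the HUD and check for win or loss.
; EndGame shows an end screen with the result and switches input to UI.
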(event Custom|AddScore
  (Math|Integer|IncrementInt (Variables|Default|GetCurrentScore)
    (:%20%20
      (Default|UpdateScore (Variables|Default|GetUIRef))
      (if (== (Variables|Default|GetCurrentScore) (Variables|Default|GetMaxScore)) ; Win check
        (CallFunction|EndGame false)))))

(event Custom|Decrement%20Time
  (bind _time (Variables|Default|GetTime))
  (if (not (Variables|Default|GetIsGameOver))
    (Math|Integer|DecrementInt _time
      (:%20%20
        (Default|UpdateCountdownText (Variables|Default|GetUIRef))
        (if (<= _time 0) ; Loss Check
          (CallFunction|EndGame true))))))

(event EventBeginPlay
  (Input|SetInputModeGameOnly (Game|GetPlayerController 0) false)
  (bind _outactors (Actor|GetAllActorsOfClass "/Game/FirstPerson/Blueprints/BP_Target.BP_Target_C"))
  (Variables|Default|SetMaxScore (Utilities|Array|Length _outactors))
  (bind _returnvalue (UserInterface|CreateWidget "/Game/FirstPerson/Blueprints/WBP_UI.WBP_UI_C"))
  (bind _output_get (Variables|Default|SetUIRef _returnvalue))
  (UserInterface|Viewport|AddtoViewport _output_get 0)
  (Default|UpdateScore _output_get)
  (Utilities|Time|SetTimerbyEvent (delegate Custom|Decrement%20Time) 0.01 true))

(fn ConstructionScript)

(fn EndGame
  (params (LostGame? :type Boolean))
  (bind _returnvalue (Game|GetPlayerController 0))
  (Variables|Default|SetIsGameOver true)
  (bind _returnvalue_2 (UserInterface|CreateWidget "/Game/FirstPerson/Blueprints/WBP_EndScreen.WBP_EndScreen_C" 0 LostGame?))
  (UserInterface|Viewport|AddtoViewport _returnvalue_2 0)
  (Input|SetInputModeUIOnly _returnvalue _returnvalue_2 "DoNotLock" false)
  (Input|SetIgnoreMoveInput _returnvalue true)
  (Variables|/Script/Engine.PlayerController|SetbShowMouseCursor _returnvalue true))