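; BP_Target is a shootable target that scores a point and gets knocked away when a BP_FirstPersonProjectile hits it.
; The first hit sets the IsNotHit flag, which despite its name marks the target as hit and blocks repeat scoring.
; It then calls AddScore on GM_TargetGame, enables physics on the Target component, and applies an impulse along the hit normal plus torque to send it flying.
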(event OnComponentHit(Target)
  (params (HitComponent :type Primitive%20Component%20Object%20Reference) (OtherActor :type Actor%20Object%20Reference) (OtherComp :type Primitive%20Component%20Object%20Reference) (NormalImpulse :type Vector :default "0, 0, 0") (Hit :type Hit%20Result%20Structure%20%28by%20ref%29))
  (bind _target (Variables|Default|GetTarget))
  (Utilities|Casting|CastToBP_FirstPersonProjectile OtherActor)
  (if (not (Variables|Default|GetIsNotHit?))
    (Variables|Default|SetIsNotHit? true)
    (bind _asgm_target_game (Utilities|Casting|CastToGM_TargetGame (Game|GetGameMode)))
    (Default|AddScore _asgm_target_game)
    (Physics|SetSimulatePhysics _target true)
    (Physics|AddImpulse _target (* (.Normal (Collision|BreakHitResult Hit)) 1e+03) "None" true)
    (Class|PrimitiveComponent|AddTorqueinRadians _target (* (Math|Vector|GetForwardVector (Variables|Default|GetTarget)) "2000.000000,0.000000,0.000000") "None" true)))

(fn ConstructionScript)